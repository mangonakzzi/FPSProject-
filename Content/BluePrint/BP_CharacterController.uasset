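; BP_CharacterController is a controller Blueprint that drives four-directional movement of the player pawn through Enhanced Input.
; BeginPlay registers the IMC_Character mapping context on player 0's local input subsystem.
; Separate W, A, S and D input actions feed movement input to player pawn 0 along yaw-only control-rotation vectors, keeping movement view-relative and independent of pitch.
; It contains no look or jump handling.
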(event `self.ReceiveBeginPlay`
  (`EnhancedInputSubsystemInterface.AddMappingContext` (pcsubsystem `EnhancedInputLocalPlayerSubsystem` (`GameplayStatics.GetPlayerController` 0)) "/Game/Input/IMC_Character.IMC_Character" 0 (struct)))

(event `EnhancedInput|/Game/Input/IA_Move_W`
  (params (ActionValue :type "Float (double-precision)") (ElapsedSeconds :type "Float (double-precision)") (TriggeredSeconds :type "Float (double-precision)") (InputAction :type "InputAction Object Reference" :default "/Game/Input/IA_Move_W.IA_Move_W"))
  (bind (_returnvalue_roll _returnvalue_pitch _returnvalue_yaw) (`KismetMathLibrary.BreakRotator` (`self.GetControlRotation`)))
  (:`Triggered`
    (`Pawn.AddMovementInput` (`GameplayStatics.GetPlayerPawn` 0) (`KismetMathLibrary.GetForwardVector` (`KismetMathLibrary.MakeRotator` 0.0 0.0 _returnvalue_yaw)) 1.0 false)))

(event `EnhancedInput|/Game/Input/IA_Move_S`
  (params (ActionValue :type "Float (double-precision)") (ElapsedSeconds :type "Float (double-precision)") (TriggeredSeconds :type "Float (double-precision)") (InputAction :type "InputAction Object Reference" :default "/Game/Input/IA_Move_S.IA_Move_S"))
  (bind (_returnvalue_roll _returnvalue_pitch _returnvalue_yaw) (`KismetMathLibrary.BreakRotator` (`self.GetControlRotation`)))
  (:`Triggered`
    (`Pawn.AddMovementInput` (`GameplayStatics.GetPlayerPawn` 0) (`KismetMathLibrary.GetForwardVector` (`KismetMathLibrary.MakeRotator` 0.0 0.0 _returnvalue_yaw)) -1.0 false)))

(event `EnhancedInput|/Game/Input/IA_Move_D`
  (params (ActionValue :type "Float (double-precision)") (ElapsedSeconds :type "Float (double-precision)") (TriggeredSeconds :type "Float (double-precision)") (InputAction :type "InputAction Object Reference" :default "/Game/Input/IA_Move_D.IA_Move_D"))
  (bind (_returnvalue_roll _returnvalue_pitch _returnvalue_yaw) (`KismetMathLibrary.BreakRotator` (`self.GetControlRotation`)))
  (:`Triggered`
    (`Pawn.AddMovementInput` (`GameplayStatics.GetPlayerPawn` 0) (`KismetMathLibrary.GetRightVector` (`KismetMathLibrary.MakeRotator` 0.0 0.0 _returnvalue_yaw)) 1.0 false)))

(event `EnhancedInput|/Game/Input/IA_Move_A`
  (params (ActionValue :type "Float (double-precision)") (ElapsedSeconds :type "Float (double-precision)") (TriggeredSeconds :type "Float (double-precision)") (InputAction :type "InputAction Object Reference" :default "/Game/Input/IA_Move_A.IA_Move_A"))
  (bind (_returnvalue_roll _returnvalue_pitch _returnvalue_yaw) (`KismetMathLibrary.BreakRotator` (`self.GetControlRotation`)))
  (:`Triggered`
    (`Pawn.AddMovementInput` (`GameplayStatics.GetPlayerPawn` 0) (`KismetMathLibrary.GetRightVector` (`KismetMathLibrary.MakeRotator` 0.0 0.0 _returnvalue_yaw)) -1.0 false)))

(fn `UserConstructionScript`)